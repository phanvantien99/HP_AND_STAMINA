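; Player stat component that tracks current and max health and stamina for BP_Player and mirrors them on its HUD bars.
; It caches the owning BP_Player at BeginPlay, and its change functions write percentages directly to the HUD widget, except IncreaseMaxStamina.
; DecreaseHealth returns true only when health was already depleted before the hit.
; IncreaseStamina divides by MaxHP rather than MaxStamina for its bar.
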(event EventBeginPlay
  (bind _asbp_player (Utilities|Casting|CastToBP_Player (Components|GetOwner)))
  (Variables|Default|SetPlayer _asbp_player))

(fn DecreaseHealth
  (params (Damage :type Float%20%28double-precision%29))
  (if (<= (Variables|Health|GetCurrent%20HP) 0.0)
    (return true)
    (else
      (bind _output_get (Variables|Health|SetCurrent%20HP (- (Variables|Health|GetCurrent%20HP) Damage)))
      (Progress|SetPercent (Variables|/Game/UI/WB_HUD.WB_HUD_C|GetHealth (Variables|/Game/Blueprint/BP_Player.BP_Player_C|GetHUD%20Widget (Variables|Default|GetPlayer))) (/ _output_get (Variables|Health|GetMax%20HP)))
      (return false))))

(fn IncreaseHealth
  (params (HP :type Float%20%28double-precision%29))
  (bind _max_hp (Variables|Health|GetMax%20HP))
  (if (< (Variables|Health|GetMax%20HP) (+ HP (Variables|Health|GetCurrent%20HP)))
    (bind _output_get (Variables|Health|SetCurrent%20HP _max_hp))
    (Progress|SetPercent (Variables|/Game/UI/WB_HUD.WB_HUD_C|GetHealth (Variables|/Game/Blueprint/BP_Player.BP_Player_C|GetHUD%20Widget (Variables|Default|GetPlayer))) (/ _output_get _max_hp))
    (else
      (bind _output_get_2 (Variables|Health|SetCurrent%20HP (+ HP (Variables|Health|GetCurrent%20HP))))
      (Progress|SetPercent (Variables|/Game/UI/WB_HUD.WB_HUD_C|GetHealth (Variables|/Game/Blueprint/BP_Player.BP_Player_C|GetHUD%20Widget (Variables|Default|GetPlayer))) (/ _output_get_2 (Variables|Health|GetMax%20HP))))))

(fn DecreaseStamina
  (params (StaminaUsed :type Float%20%28double-precision%29))
  (if (> (Variables|Health|GetCurrent%20HP) 0.0)
    (bind _output_get (Variables|Stamina|SetCurrent%20Stamina (- (Variables|Stamina|GetCurrent%20Stamina) StaminaUsed)))
    (Progress|SetPercent (Variables|/Game/UI/WB_HUD.WB_HUD_C|GetStamina (Variables|/Game/Blueprint/BP_Player.BP_Player_C|GetHUD%20Widget (Variables|Default|GetPlayer))) (/ _output_get (Variables|Stamina|GetMax%20Stamina)))
    (else
      (bind _output_get_2 (Variables|Stamina|SetCurrent%20Stamina 0.0))
      (Progress|SetPercent (Variables|/Game/UI/WB_HUD.WB_HUD_C|GetStamina (Variables|/Game/Blueprint/BP_Player.BP_Player_C|GetHUD%20Widget (Variables|Default|GetPlayer))) (/ _output_get_2 (Variables|Stamina|GetMax%20Stamina))))))

(fn IncreaseStamina
  (params (AddedStamina :type Float%20%28double-precision%29))
  (if (> (Variables|Health|GetCurrent%20HP) 0.0)
    (if (<= (+ (Variables|Stamina|GetCurrent%20Stamina) AddedStamina) (Variables|Stamina|GetMax%20Stamina))
      (bind _output_get (Variables|Stamina|SetCurrent%20Stamina (+ (Variables|Stamina|GetCurrent%20Stamina) AddedStamina)))
      (Progress|SetPercent (Variables|/Game/UI/WB_HUD.WB_HUD_C|GetStamina (Variables|/Game/Blueprint/BP_Player.BP_Player_C|GetHUD%20Widget (Variables|Default|GetPlayer))) (/ _output_get (Variables|Health|GetMax%20HP)))
      (else
        (bind _output_get_2 (Variables|Stamina|SetCurrent%20Stamina (Variables|Stamina|GetMax%20Stamina)))
        (Progress|SetPercent (Variables|/Game/UI/WB_HUD.WB_HUD_C|GetStamina (Variables|/Game/Blueprint/BP_Player.BP_Player_C|GetHUD%20Widget (Variables|Default|GetPlayer))) (/ _output_get_2 (Variables|Health|GetMax%20HP)))))))

(fn IncreaseMaxStamina
  (params (AddedStamina :type Float%20%28double-precision%29))
  (Variables|Stamina|SetMax%20Stamina (+ AddedStamina (Variables|Stamina|GetMax%20Stamina))))

(fn IncreaseMaxHealth
  (params (HealthToIncrease :type Float%20%28double-precision%29))
  (bind _output_get (Variables|Health|SetMax%20HP (+ HealthToIncrease (Variables|Health|GetMax%20HP))))
  (Progress|SetPercent (Variables|/Game/UI/WB_HUD.WB_HUD_C|GetHealth (Variables|/Game/Blueprint/BP_Player.BP_Player_C|GetHUD%20Widget (Variables|Default|GetPlayer))) (/ (Variables|Health|GetCurrent%20HP) _output_get)))

(fn UpdateStat
  (bind _player (Variables|Default|GetPlayer))
  (bind _hud_widget (Variables|/Game/Blueprint/BP_Player.BP_Player_C|GetHUD%20Widget _player))
  (Utilities|FlowControl|Sequence
    (:then_0
      (Progress|SetPercent (Variables|/Game/UI/WB_HUD.WB_HUD_C|GetHealth _hud_widget) (/ (Variables|Health|GetCurrent%20HP) (Variables|Health|GetMax%20HP))))
    (:then_1
      (Progress|SetPercent (Variables|/Game/UI/WB_HUD.WB_HUD_C|GetStamina _hud_widget) (/ (Variables|Stamina|GetCurrent%20Stamina) (Variables|Stamina|GetMax%20Stamina))))))